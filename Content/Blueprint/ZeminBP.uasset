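; ZeminBP is a self-replacing ground segment (zemin) actor, apparently a tile in an endless track.
; When AnaCharacter overlaps SonCollission, it calls YeniZeminOlustur on AnaGameMode to create new ground, then destroys itself one second later.
; The construction script adds a child actor component at a random point computed from the SpawnNoktası box's world location and extent.
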(event `self.SonCollission.OnComponentBeginOverlap`
  (params (OverlappedComponent :type "PrimitiveComponent Object Reference") (OtherActor :type "Actor Object Reference") (OtherComp :type "PrimitiveComponent Object Reference") (OtherBodyIndex :type Integer) (bFromSweep :type Boolean) (SweepResult :type "HitResult Structure (by ref)"))
  (cast `/Game/Blueprint/AnaCharacter` OtherActor)
  (bind _asana_game_mode (cast `/Game/Blueprint/AnaGameMode` (`GameplayStatics.GetGameMode`)))
  (`/Game/Blueprint/AnaGameMode.YeniZeminOlustur` _asana_game_mode)
  (`KismetSystemLibrary.Delay` 1.0)
  (`self.K2_DestroyActor`))

(fn `UserConstructionScript`
  (bind `_spawnnoktası` (`self.SpawnNoktası`))
  (`AddComponent|NODE_AddChildActorComponent-0` :`bManualAttachment` true :`RelativeTransform` (`KismetMathLibrary.MakeTransform` (`KismetMathLibrary.RandomPointInBoundingBox` (`SceneComponent.K2_GetComponentLocation` `_spawnnoktası`) (`BoxComponent.BoxExtent` `_spawnnoktası`)) (struct) (1.0 1.0 1.0))))